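; BP_CodePanel is a level-placeable code puzzle made of five child-actor code hexagons that must match a WinningCode.
; On BeginPlay it passes the code to a linked CodePanelHiddenSolution, gathers the hexagons and binds their side-change events, printing an error if the link is missing.
; Each change rechecks every hexagon's side, and the first full match notifies the Flow graph on authority with a solved tag.
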(event Custom|AdjustHint
  (bind _codepanelhiddensolution (Variables|CodePanel|GetCodePanelHiddenSolution)
    (:then
      (Default|AdjustSolution _codepanelhiddensolution (Variables|CodePanel|GetWinningCode)))
    (:else
      (Development|PrintString "Error: BP_CodePanel must have a valid CodePanelHiddenSolution!" true true "(R=1.000000,G=0.000000,B=0.016666,A=1.000000)"))))

(event Custom|HandleOnCurrentSideChanged
  (params (Hex :type BP%20Code%20Hexagon%20Object%20Reference) (NewSide :type E_HexagonSide%20Enum :default "NewEnumerator0"))
  (bind _bwon (CodePanel|CheckforWinningCode))
  (if _bwon
    (Utilities|FlowControl|DoOnce false
      (:Completed
        (Class|FlowComponent|NotifyGraph (Variables|Default|GetFlow) (Variables|CodePanel|GetNotifyPanelSolvedTag) "Authority")
        (Development|PrintString "Code panel solved!")))))

(event EventBeginPlay
  (bind _codepanelhiddensolution (Variables|CodePanel|GetCodePanelHiddenSolution)
    (:then
      (Default|AdjustSolution _codepanelhiddensolution (Variables|CodePanel|GetWinningCode))
      (for (_array_element _array_index) (Utilities|Array|MakeArray (Variables|Default|GetCodeHex1) (Variables|Default|GetCodeHex2) (Variables|Default|GetCodeHex3) (Variables|Default|GetCodeHex4) (Variables|Default|GetCodeHex5))
        (Utilities|Array|SetArrayElem (Variables|CodePanel|GetHexArray) _array_index (.AsBP%20Code%20Hexagon (Utilities|Casting|CastToBP_CodeHexagon (Variables|/Script/Engine.ChildActorComponent|GetChildActor _array_element))) true)
        (EventDispatchers|BindEventtoOnCurrentSideChanged (.AsBP%20Code%20Hexagon (Utilities|Casting|CastToBP_CodeHexagon (Variables|/Script/Engine.ChildActorComponent|GetChildActor _array_element))) (delegate Custom|HandleOnCurrentSideChanged))))
    (:else
      (Development|PrintString "Error: BP_CodePanel must have a valid CodePanelHiddenSolution!" true true "(R=1.000000,G=0.000000,B=0.016666,A=1.000000)"))))

(fn ConstructionScript)

(fn CheckforWinningCode
  (for (_array_element _array_index) (Variables|CodePanel|GetHexArray)
    (if (Utilities|Enum|NotEqual(Enum) (Default|GetCurrentSide _array_element) (Utilities|Array|Get(acopy) (Variables|CodePanel|GetWinningCode) _array_index))
      (return false)))
  (return true))