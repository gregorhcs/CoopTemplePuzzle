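; BP_CodePanelHiddenSolution is a placeable level-logic actor with six hex components, apparently meant to display a code panel's solution.
; AdjustSolution takes a Solution array but its entry is unwired, so it currently does nothing.
; Its disconnected loop would look up each element in SideMaterialMapping and apply a dynamic material instance to the hex at that index.
; BeginPlay and the construction script are empty.
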(event EventBeginPlay)

(fn ConstructionScript)

(fn AdjustSolution
  (params (Solution :type Array%20of%20E_HexagonSide%20Enums :default "NewEnumerator0")))