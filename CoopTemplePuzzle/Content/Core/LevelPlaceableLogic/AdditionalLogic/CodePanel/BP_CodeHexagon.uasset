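; Interactable six-sided hexagon dial, likely one element of a code panel puzzle.
; Interacting calls RotateUp, which advances the side index with wraparound, turns the mesh 60 degrees and broadcasts the new side enum through OnCurrentSideChanged.
; RotateDown decrements the index but turns the mesh in the same direction as RotateUp.
; BeginPlay gathers the six side variables into a Sides array, unused elsewhere in this Blueprint.
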(event OnStartInteract(BC_Interactable)
  (params (Interactor :type BC%20Interactor%20Object%20Reference))
  (CodeHexagon|RotateUp))

(event EventBeginPlay
  (Variables|CodeHexagon|SetSides (Utilities|Array|MakeArray (Variables|Default|GetSide1) (Variables|Default|GetSide2) (Variables|Default|GetSide3) (Variables|Default|GetSide4) (Variables|Default|GetSide5) (Variables|Default|GetSide6))))

(fn ConstructionScript)

(fn RotateUp
  (Variables|CodeHexagon|SetCurrentSide (Math|Integer|%(Integer) (+ (Variables|CodeHexagon|GetCurrentSide) 1) 6))
  (Transformation|AddLocalRotation (Variables|Default|GetStaticMesh) "0.000000,0.000000,-60.000000" false false)
  (Default|CallOnCurrentSideChanged self (CodeHexagon|GetCurrentSide)))

(fn RotateDown
  (Variables|CodeHexagon|SetCurrentSide (Math|Integer|SelectInt (- (Variables|CodeHexagon|GetCurrentSide) 1) 5 (>= (- (Variables|CodeHexagon|GetCurrentSide) 1) 0)))
  (Transformation|AddLocalRotation (Variables|Default|GetStaticMesh) "0.000000,0.000000,-60.000000" false false)
  (Default|CallOnCurrentSideChanged self (CodeHexagon|GetCurrentSide)))

(fn GetCurrentSide
  (return (Utilities|Select :Index (Variables|CodeHexagon|GetCurrentSide) :Option%200 "NewEnumerator0" :Option%201 "NewEnumerator1" :Option%202 "NewEnumerator2" :Option%203 "NewEnumerator3" :Option%204 "NewEnumerator4" :Option%205 "NewEnumerator5")))