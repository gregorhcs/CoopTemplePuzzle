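; BP_TriggerVolume is a trigger actor that links player-space overlaps to a puzzle Flow graph, apparently as a test.
; The first actor overlap, gated by DoOnce, notifies the graph through its Flow component with an entered-test-area tag on authority.
; When the component receives a notify back, it prints a debug message and plays a timeline that offsets the Sphere's relative Z from its current height.
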(event ReceiveNotify(Flow)
  (params (FlowComponent :type Flow%20Component%20Object%20Reference) (NotifyTag :type Gameplay%20Tag%20Structure%20%28by%20ref%29))
  (bind _sphere (Variables|Default|GetSphere))
  (bind _relativelocation (Variables|/Script/Engine.SceneComponent|GetRelativeLocation _sphere))
  (Variables|Default|SetReturn%20Value%20Z (.z _relativelocation))
  (Development|PrintString "Notify")
  (bind _newtrack_0 (Timeline|Timeline PlayFromStart)
    (:Update
      (Transformation|SetRelativeLocation (Variables|Default|GetSphere) (Math|Vector|MakeVector (.x _relativelocation) (.y _relativelocation) (+ (* _newtrack_0 1e+02) (Variables|Default|GetReturn%20Value%20Z))) false false))))

(event Collision|EventActorBeginOverlap
  (params (OtherActor :type Actor%20Object%20Reference))
  (Utilities|FlowControl|DoOnce false
    (:Completed
      (Class|FlowComponent|NotifyGraph (Variables|Default|GetFlow) "(TagName=\"Puzzle.Flow.EnteredTestArea\")" "Authority"))))

(fn ConstructionScript)