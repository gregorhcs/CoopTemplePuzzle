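; BP_TriggerVolume is a puzzle-system trigger actor that moves its Sphere component in response to Flow notify tags.
; The "Go Sideways" and "Go Up" tags each cache the sphere's relative Y or Z, then run a timeline that offsets that axis by the scaled curve value.
; Go Sideways uses Play, while Go Up restarts from the start and prints a debug string.
; GetOverlapCollider supplies OverlapBox as the overlap collider.
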(event ReceiveNotify(Flow)
  (params (FlowComponent :type Flow%20Component%20Object%20Reference) (NotifyTag :type Gameplay%20Tag%20Structure%20%28by%20ref%29))
  (bind _sphere (Variables|Default|GetSphere))
  (bind _sphere_2 (Variables|Default|GetSphere))
  (bind _relativelocation (Variables|/Script/Engine.SceneComponent|GetRelativeLocation _sphere))
  (bind _relativelocation_2 (Variables|/Script/Engine.SceneComponent|GetRelativeLocation _sphere_2))
  (|SwitchGameplayTag NotifyTag
    (:Puzzle.NotifiesToActor.GoSideways
      (Variables|Default|SetRelative%20Location%20Y (.y _relativelocation))
      (bind _newtrack_0 (Timeline|Timeline_0 Play)
        (:Update
          (Transformation|SetRelativeLocation (Variables|Default|GetSphere) (Math|Vector|MakeVector (.x _relativelocation) (+ (* _newtrack_0 1e+02) (Variables|Default|GetRelative%20Location%20Y)) (.z _relativelocation)) false false))))
    (:Puzzle.NotifiesToActor.GoUp
      (Variables|Default|SetReturn%20Value%20Z (.z _relativelocation_2))
      (Development|PrintString "Notify")
      (bind _newtrack_0_2 (Timeline|Timeline PlayFromStart)
        (:Update
          (Transformation|SetRelativeLocation (Variables|Default|GetSphere) (Math|Vector|MakeVector (.x _relativelocation_2) (.y _relativelocation_2) (+ (* _newtrack_0_2 1e+02) (Variables|Default|GetReturn%20Value%20Z))) false false))))))

(fn ConstructionScript)

(fn GetOverlapCollider
  (return (Variables|Default|GetOverlapBox)))